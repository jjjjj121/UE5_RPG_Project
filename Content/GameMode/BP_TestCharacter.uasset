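; Test player character Blueprint that forwards damage to the HUD and hosts debug hotkeys.
; ReceivingDamage passes max and current HP to the BP_W_HUD widget.
; Number keys switch the weapon enum with montage calls, toggle walk speed, trigger death, and print debug text or location.
; A macro buckets hit angle into four directional reaction indices; camera-trace, weapon-attach and widget experiments sit disconnected.
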(event EventTick
  (params (DeltaSeconds :type Float%20%28single-precision%29)))

(event EventReceivingDamage
  (params (MaxHP :type Float%20%28single-precision%29) (CurHP :type Float%20%28single-precision%29))
  (bind _hud (Variables|Default|GetHUD)
    (:then
      (bind _asbp_w_hud (Utilities|Casting|CastToBP_W_HUD (Variables|/Script/RPGGame.RPGGameHUD|GetHUDWidget _hud)))
      (Default|WUpdateHP _asbp_w_hud MaxHP CurHP))
    (:else)))

(event Input|MouseEvents|RightMouseButton
  (params (Key :type Key%20Structure :default "None")))

(event EventBeginPlay)

(event Input|KeyboardEvents|4
  (params (Key :type Key%20Structure))
  (bind _returnvalue (Transformation|GetActorLocation))
  (:Pressed
    (Development|PrintString (Utilities|String|Append "Character x :     " (Utilities|String|ToString(Float) (.x _returnvalue)) "y :    " (Utilities|String|ToString(Float) (.y _returnvalue)) "z :   " (Utilities|String|ToString(Float) (.z _returnvalue))) true true "(R=0.000000,G=0.660000,B=1.000000,A=1.000000)" 5e+01)))

(event Input|KeyboardEvents|0
  (params (Key :type Key%20Structure))
  (:Pressed
    (Variables|Default|SetWeaponEnum "Hand")
    (Animation|PlayAnimMontage 0 0.7 "None")))

(event Input|KeyboardEvents|1
  (params (Key :type Key%20Structure))
  (:Pressed
    (Variables|Default|SetWeaponEnum "GreatSword")
    (Animation|PlayAnimMontage 0 1.0 "None")))

(event Input|KeyboardEvents|3
  (params (Key :type Key%20Structure))
  (:Pressed
    (Utilities|FlowControl|FlipFlop
      (:A
        (Variables|/Script/Engine.CharacterMovementComponent|SetMaxWalkSpeed (Variables|Character|GetCharacterMovement) 2e+02))
      (:B
        (Variables|/Script/Engine.CharacterMovementComponent|SetMaxWalkSpeed (Variables|Character|GetCharacterMovement) 4.5e+02)))))

(event Input|KeyboardEvents|2
  (params (Key :type Key%20Structure))
  (:Pressed
    (Development|PrintString "Hello")))

(event Input|KeyboardEvents|5
  (params (Key :type Key%20Structure))
  (:Pressed
    (Class|RPGGameCharacter|DoDeath 1)))

(fn ConstructionScript)